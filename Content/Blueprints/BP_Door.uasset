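; BP_Door is a sliding door that opens when the player character enters its collision box and closes when they leave.
; Overlap events play and reverse the AnimateDoor timeline, whose track interpolates the door's relative location between stored begin and end vectors.
; OpenDoor and CloseDoor events drive the same timeline, so the door can also be triggered directly.
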(event `OpenDoor`
  (bind (_direction _dore) (`Timeline|Animate Door` :!label _label)
    (:`Update`
      (`SceneComponent.K2_SetRelativeLocation` (`self.Door`) (`KismetMathLibrary.VLerp` (`self.DoorLocBegin`) (`self.DoorLocEnd`) _dore) false false))))

(event `self.CollisionBox.OnComponentBeginOverlap`
  (params (OverlappedComponent :type "PrimitiveComponent Object Reference") (OtherActor :type "Actor Object Reference") (OtherComp :type "PrimitiveComponent Object Reference") (OtherBodyIndex :type Integer) (bFromSweep :type Boolean) (SweepResult :type "HitResult Structure (by ref)"))
  (if (== OtherActor (`GameplayStatics.GetPlayerCharacter` 0))
    (goto _label)))

(event `CloseDoor`
  (goto _label :!via `Reverse`))

(event `self.CollisionBox.OnComponentEndOverlap`
  (params (OverlappedComponent :type "PrimitiveComponent Object Reference") (OtherActor :type "Actor Object Reference") (OtherComp :type "PrimitiveComponent Object Reference") (OtherBodyIndex :type Integer))
  (if (== OtherActor (`GameplayStatics.GetPlayerCharacter` 0))
    (goto _label :!via `Reverse`)))

(fn `UserConstructionScript`)